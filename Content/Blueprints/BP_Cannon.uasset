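; BP_Cannon is a cannon actor that automatically fires a cannonball every second from BeginPlay onward.
; A looping Delay calls FireCannon, which prints the running shot number and spawns a BP_CannonBall at the Spawnpoint transform.
; It launches each ball by applying a large acceleration-based force to its Cube along the Spawnpoint's forward vector, then increments the shot counter.
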(event Custom|FireCannon
  (Development|PrintText (Utilities|Text|FormatText "Firing cannonball number {count}!" (Variables|Default|GetShotcount)) true true "(R=0.000000,G=0.660000,B=1.000000,A=1.000000)" 1.0)
  (bind _returnvalue (Game|SpawnActorfromClass "/Game/Blueprints/BP_CannonBall.BP_CannonBall_C" (Transformation|GetWorldTransform (Variables|Default|GetSpawnpoint)) "Undefined" "MultiplyWithRoot" 0 0)) ; spawn actor from class
  (Physics|AddForce (Variables|/Game/Blueprints/BP_CannonBall.BP_CannonBall_C|GetCube _returnvalue) (* (Math|Vector|GetForwardVector (Variables|Default|GetSpawnpoint)) 1e+05) "None" true)
  (Math|Integer|IncrementInt (Variables|Default|GetShotcount)))

(event EventBeginPlay
  (Utilities|FlowControl|Delay 1.0 :!label _label)
  (CallFunction|FireCannon)
  (goto _label))

(fn ConstructionScript)