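; BP_DialogueManager shows lines from a Dialogue array one at a time through an on-screen widget.
; It creates a W_Dialogue widget on BeginPlay and stores it for reuse.
; DisplayNextLine sets the widget text, also prints the line, and keeps the widget in the viewport for a timed delay.
; A Sequence advances the index without waiting for that delay, and the index wraps to the first line past the end.
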(event Custom|DisplayNextLine
  (bind _dialoguewidget (Variables|Default|GetDialogueWidget))
  (if (>= (Variables|Default|GetIndex) (Utilities|Array|Length (Variables|Default|GetDialogue))) ; if the index is greater than\nor equal to the lenth of the \nDialogue Array, reset it.
    (Variables|Default|SetIndex 0))
  (Development|PrintText (Utilities|Array|Get(acopy) (Variables|Default|GetDialogue) (Variables|Default|GetIndex)) true true "(R=0.000000,G=0.070267,B=1.000000,A=1.000000)" 5.0)
  (Rendering|Components|TextRender|SetText (Variables|/Game/Widget/W_Dialogue.W_Dialogue_C|GetTextBlock_0 (Variables|Default|GetDialogueWidget)) (Utilities|Array|Get(acopy) (Variables|Default|GetDialogue) (Variables|Default|GetIndex)))
  (Utilities|FlowControl|Sequence
    (:then_0
      (UserInterface|Viewport|AddtoViewport _dialoguewidget 0)
      (Utilities|FlowControl|Delay 5.0)
      (Widget|RemovefromParent _dialoguewidget))
    (:then_1
      (Math|Integer|IncrementInt (Variables|Default|GetIndex)) ; increment Int\nto add 1 to our index
    )))

(event EventBeginPlay
  (bind _returnvalue (UserInterface|CreateWidget "/Game/Widget/W_Dialogue.W_Dialogue_C")) ; "Create Widget"
  (Variables|Default|SetDialogueWidget _returnvalue))

(fn ConstructionScript)