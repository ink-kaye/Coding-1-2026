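; BP_LoreBook is a dungeon-piece book the player can read up close, shown as an on-screen widget.
; A Box overlap tracks whether BP_ThirdPersonCharacter is close enough, gating the UseOpenClose event that toggles reading.
; Picking up creates the widget and adds it to the viewport, while putting down removes it.
; Leaving the box also puts the book down automatically.
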(event OnComponentEndOverlap(Box)
  (params (OverlappedComponent :type Primitive%20Component%20Object%20Reference) (OtherActor :type Actor%20Object%20Reference) (OtherComp :type Primitive%20Component%20Object%20Reference) (OtherBodyIndex :type Integer))
  (Utilities|Casting|CastToBP_ThirdPersonCharacter OtherActor)
  (CallFunction|PutDownBook)
  (Variables|Default|SetIsCloseEnough? false))

(event OnComponentBeginOverlap(Box)
  (params (OverlappedComponent :type Primitive%20Component%20Object%20Reference) (OtherActor :type Actor%20Object%20Reference) (OtherComp :type Primitive%20Component%20Object%20Reference) (OtherBodyIndex :type Integer) (bFromSweep :type Boolean) (SweepResult :type Hit%20Result%20Structure%20%28by%20ref%29))
  (Utilities|Casting|CastToBP_ThirdPersonCharacter OtherActor)
  (Variables|Default|SetIsCloseEnough? true))

(event Custom|PutDownBook
  (Widget|RemovefromParent (stale Custom|PickupBook _returnvalue))
  (Variables|Default|SetIsReading? false))

(event Custom|TogglePickup
  (if (Variables|Default|GetIsReading?)
    (CallFunction|PutDownBook)
    (else
      (CallFunction|PickupBook))))

(event Custom|PickupBook
  (bind _returnvalue (UserInterface|CreateWidget (Variables|Default|GetClass)))
  (UserInterface|Viewport|AddtoViewport _returnvalue 0)
  (Variables|Default|SetIsReading? true))

(event EventBeginPlay)

(event Collision|EventActorBeginOverlap
  (params (OtherActor :type Actor%20Object%20Reference)))

(event EventTick
  (params (DeltaSeconds :type Float%20%28single-precision%29)))

(event EventUseOpenClose
  (if (Variables|Default|GetIsCloseEnough?)
    (CallFunction|TogglePickup)))

(fn ConstructionScript)