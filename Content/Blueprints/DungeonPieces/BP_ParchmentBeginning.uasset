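; Readable parchment note for the dungeon that shows its text in an on-screen journal widget when the player interacts.
; Actor overlap prints an F-key hint, while the Box overlap gates UseOpenClose, which toggles reading.
; Each pickup creates a W_ParchmentPickupBP, shows the next Text array entry and cycles the page index.
; The widget closes on toggle, leaving the box or a timed delay, though the delay leaves IsReading set.
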(event OnComponentEndOverlap(Box)
  (params (OverlappedComponent :type Primitive%20Component%20Object%20Reference) (OtherActor :type Actor%20Object%20Reference) (OtherComp :type Primitive%20Component%20Object%20Reference) (OtherBodyIndex :type Integer))
  (Utilities|Casting|CastToBP_ThirdPersonCharacter OtherActor)
  (CallFunction|PutDownParchment)
  (Variables|Default|SetIsCloseEnough? false))

(event OnComponentBeginOverlap(Box)
  (params (OverlappedComponent :type Primitive%20Component%20Object%20Reference) (OtherActor :type Actor%20Object%20Reference) (OtherComp :type Primitive%20Component%20Object%20Reference) (OtherBodyIndex :type Integer) (bFromSweep :type Boolean) (SweepResult :type Hit%20Result%20Structure%20%28by%20ref%29))
  (Utilities|Casting|CastToBP_ThirdPersonCharacter OtherActor)
  (Variables|Default|SetIsCloseEnough? true))

(event Custom|DisplayNextLine
  (if (>= (Variables|Default|GetPage%20Counter) (Utilities|Array|Length (Variables|Default|GetText)))
    (Variables|Default|SetPage%20Counter 0))
  (Development|PrintText (Utilities|Array|Get(acopy) (Variables|Default|GetText) (Variables|Default|GetPage%20Counter)) true true "(R=0.000000,G=0.070267,B=1.000000,A=1.000000)" 5.0)
  (Rendering|Components|TextRender|SetText (Variables|/Game/Widget/W_ParchmentPickupBP.W_ParchmentPickupBP_C|GetTextInJournal (Variables|Default|GetNoteText)) (Utilities|Array|Get(acopy) (Variables|Default|GetText) (Variables|Default|GetPage%20Counter)))
  (Utilities|FlowControl|Sequence
    (:then_0
      (Utilities|FlowControl|Delay 15.0)
      (Widget|RemovefromParent (Variables|Default|GetNoteText)))
    (:then_1
      (Math|Integer|IncrementInt (Variables|Default|GetPage%20Counter)) ; increment Int\nto add 1 to our index
    )))

(event Custom|TogglePickup
  (if (Variables|Default|GetisReading?)
    (CallFunction|PutDownParchment)
    (else
      (CallFunction|PickupParchment))))

(event Custom|PutDownParchment
  (Widget|RemovefromParent (stale Custom|PickupParchment _returnvalue))
  (Variables|Default|SetisReading? false))

(event Custom|PickupParchment
  (bind _returnvalue (UserInterface|CreateWidget "/Game/Widget/W_ParchmentPickupBP.W_ParchmentPickupBP_C"))
  (Variables|Default|SetNoteText _returnvalue)
  (UserInterface|Viewport|AddtoViewport (Variables|Default|GetNoteText) 0)
  (Variables|Default|SetisReading? true)
  (CallFunction|DisplayNextLine))

(event Collision|EventActorBeginOverlap
  (params (OtherActor :type Actor%20Object%20Reference))
  (Utilities|Casting|CastToBP_ThirdPersonCharacter OtherActor)
  (Development|PrintText "Press F to Interact with Notes and Books!"))

(event EventUseOpenClose
  (if (Variables|Default|GetIsCloseEnough?)
    (CallFunction|TogglePickup)))

(fn ConstructionScript)