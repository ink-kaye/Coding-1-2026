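; BP_LoreBook1 is a dungeon lore book that the player can read as an on-screen widget when standing close to it.
; A Box overlap with BP_ThirdPersonCharacter sets the proximity flag that gates the UseOpenClose event.
; That event toggles reading by creating the widget in the viewport or removing it.
; Leaving the box also removes the widget and clears the proximity flag.
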(event OnComponentEndOverlap(Box)
  (params (OverlappedComponent :type Primitive%20Component%20Object%20Reference) (OtherActor :type Actor%20Object%20Reference) (OtherComp :type Primitive%20Component%20Object%20Reference) (OtherBodyIndex :type Integer))
  (Utilities|Casting|CastToBP_ThirdPersonCharacter OtherActor)
  (CallFunction|PutDownParchment)
  (Variables|Default|SetIs%20Close%20Enough? false))

(event OnComponentBeginOverlap(Box)
  (params (OverlappedComponent :type Primitive%20Component%20Object%20Reference) (OtherActor :type Actor%20Object%20Reference) (OtherComp :type Primitive%20Component%20Object%20Reference) (OtherBodyIndex :type Integer) (bFromSweep :type Boolean) (SweepResult :type Hit%20Result%20Structure%20%28by%20ref%29))
  (Utilities|Casting|CastToBP_ThirdPersonCharacter OtherActor)
  (Variables|Default|SetIs%20Close%20Enough? true))

(event Custom|TogglePickup
  (if (Variables|Default|GetIs%20Reading?)
    (CallFunction|PutDownParchment)
    (else
      (CallFunction|PickupParchment))))

(event Custom|PutDownParchment
  (Widget|RemovefromParent (stale Custom|PickupParchment _returnvalue))
  (Variables|Default|SetIs%20Reading? false))

(event Custom|PickupParchment
  (bind _returnvalue (UserInterface|CreateWidget (Variables|Default|GetClass)))
  (UserInterface|Viewport|AddtoViewport _returnvalue 0)
  (Variables|Default|SetIs%20Reading? true))

(event EventBeginPlay)

(event Collision|EventActorBeginOverlap
  (params (OtherActor :type Actor%20Object%20Reference)))

(event EventTick
  (params (DeltaSeconds :type Float%20%28single-precision%29)))

(event EventUseOpenClose
  (if (Variables|Default|GetIs%20Close%20Enough?)
    (CallFunction|TogglePickup)))

(fn ConstructionScript)