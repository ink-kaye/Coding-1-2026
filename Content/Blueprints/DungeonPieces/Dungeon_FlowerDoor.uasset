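; Dungeon door Blueprint that stays locked until the player character brings a Flower Key.
; On actor overlap it casts to BP_ThirdPersonCharacter, prints a locked message and checks that character's FlowerKey count.
; With a key, it decrements the count and destroys the gate door and both box components, leaving the actor itself in place.
; Without one, it prints a hint to find the key.
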(event EventBeginPlay)

(event Collision|EventActorBeginOverlap
  (params (OtherActor :type Actor%20Object%20Reference))
  (bind _asbp_third_person_character (Utilities|Casting|CastToBP_ThirdPersonCharacter OtherActor))
  (Development|PrintText "The Flower door is locked. ")
  (if (> (Variables|/Game/ThirdPerson/Blueprints/BP_ThirdPersonCharacter.BP_ThirdPersonCharacter_C|GetFlowerKey _asbp_third_person_character) 0)
    (Math|Integer|DecrementInt (Variables|/Game/ThirdPerson/Blueprints/BP_ThirdPersonCharacter.BP_ThirdPersonCharacter_C|GetFlowerKey _asbp_third_person_character)
      (:%20%20
        (Components|DestroyComponent (Variables|Default|Getgate-door))
        (Components|DestroyComponent (Variables|Default|GetBox))
        (Components|DestroyComponent (Variables|Default|GetBox1))))
    (else
      (Development|PrintText "You must find the Flower Key to unlock this door."))))

(event EventTick
  (params (DeltaSeconds :type Float%20%28single-precision%29)))

(fn ConstructionScript)